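; BP_CatController is a player controller that switches between a cursorless cat mode and a box mode where items are dragged with the mouse.
; While the cursor shows, left click picks a BP_Item under it by visibility trace and moves it to the impact point on WorldStatic objects under the cursor.
; Releasing the click records the item and its location in the BP_MiniCat save game object, then clears the dragged item.
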(event `CatMode`
  (set `self.bShowMouseCursor` false))

(event `BoxMode`
  (set `self.bShowMouseCursor` true))

(event `EnhancedInput|/Game/Template/ThirdPerson/Input/Actions/IA_LeftClick`
  (params (ActionValue :type Boolean) (ElapsedSeconds :type "Float (double-precision)") (TriggeredSeconds :type "Float (double-precision)") (InputAction :type "InputAction Object Reference" :default "/Game/Template/ThirdPerson/Input/Actions/IA_LeftClick.IA_LeftClick"))
  (bind _draggeditem (`self.DraggedItem`))
  (bind (_bblockinghit _binitialoverlap _time _distance _location _impactpoint _normal _impactnormal _physmat _hitactor) (`GameplayStatics.BreakHitResult` (`self.GetHitResultUnderCursorByChannel` "TraceTypeQuery1")))
  (bind (_bblockinghit_2 _binitialoverlap_2 _time_2 _distance_2 _location_2 _impactpoint_2) (`GameplayStatics.BreakHitResult` (`self.GetHitResultUnderCursorForObjects` (`|MakeArray` "ObjectTypeQuery1" :!type "EObjectTypeQuery Enum"))))
  (:`Triggered`
    (if (`self.bShowMouseCursor`)
      (`self.DraggedItem`
        (:`then`
          (if _bblockinghit_2 :!label _label
            (`self.K2_SetActorLocation` (`self.DraggedItem`) _impactpoint_2 false false)))
        (:`else`
          (if _bblockinghit
            (bind _asbp_item (cast `/Game/Boxcat/Items/BP_Item` _hitactor))
            (set `self.DraggedItem` _asbp_item)
            (goto _label))))))
  (:`Completed`
    (bind _asbp_mini_cat (cast `/Game/Boxcat/Cat/BP_MiniCat` (`GameplayStatics.GetPlayerCharacter` 0)))
    (`BlueprintMapLibrary.Map_Add` (`/Game/Boxcat/SaveGame/BP_SaveGame.PlacedItems` (`/Game/Boxcat/Cat/BP_Cat.BP_SaveGame` _asbp_mini_cat)) _draggeditem (`self.K2_GetActorLocation` _draggeditem))
    (set `self.DraggedItem` null)))

(fn `UserConstructionScript`)