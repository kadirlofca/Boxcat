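; BP_MiniCat is a cat Blueprint that restores saved items into the level on BeginPlay.
; It respawns each placed item as a BP_Item at its saved location, setting the mesh from its item enum.
; It then spawns inventory items at the BP_InventoryItemSpawner, nudged clear of collisions where possible.
; Those items are recorded as placed at the spawner's location, the inventory is cleared and the save is written.
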(event `LoadPlacedItems`
  (for _array_element (`/Game/Boxcat/SaveGame/BP_SaveGame.PlacedItems` (`self.BP_SaveGame`))
    (bind _returnvalue (`|SpawnActorFromClass` "/Game/Boxcat/Items/BP_Item.BP_Item_C" (`KismetMathLibrary.MakeTransform` (`.Location_5_37C261C845730CBA148377A33A2DD256` (break `/Game/Boxcat/Items/S_PlacedItems` _array_element))) "AlwaysSpawn" "MultiplyWithRoot" null null))
    (`/Game/Boxcat/Items/BP_Item.SetMeshFromEnum` _returnvalue (break `/Game/Boxcat/Items/S_PlacedItems` _array_element))))

(event `SpawnInventoryItems`
  (bind _bp_savegame (`self.BP_SaveGame`))
  (bind _itemsininventory (`/Game/Boxcat/SaveGame/BP_SaveGame.ItemsInInventory` _bp_savegame))
  (bind _returnvalue (`GameplayStatics.GetActorOfClass` "/Game/Boxcat/Box/BP_InventoryItemSpawner.BP_InventoryItemSpawner_C"))
  (for _array_element _itemsininventory
    (bind _returnvalue_2 (`self.K2_GetActorLocation` _returnvalue))
    (bind _returnvalue_3 (`|SpawnActorFromClass` "/Game/Boxcat/Items/BP_Item.BP_Item_C" (`KismetMathLibrary.MakeTransform` _returnvalue_2) "AdjustIfPossibleButAlwaysSpawn" "MultiplyWithRoot" null null))
    (`/Game/Boxcat/Items/BP_Item.SetMeshFromEnum` _returnvalue_3 _array_element)
    (`KismetArrayLibrary.Array_Add` (`/Game/Boxcat/SaveGame/BP_SaveGame.PlacedItems` _bp_savegame) (make `/Game/Boxcat/Items/S_PlacedItems` _array_element _returnvalue_2)))
  (`KismetArrayLibrary.Array_Clear` _itemsininventory)
  (`GameplayStatics.SaveGameToSlot` _bp_savegame "save1"))

(event `self.ReceiveBeginPlay`
  (`parent.ReceiveBeginPlay`)
  (`self.LoadPlacedItems`)
  (`self.SpawnInventoryItems`))

(fn `UserConstructionScript`
  (`parent.UserConstructionScript`))