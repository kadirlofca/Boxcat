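; BP_CatCamera is a follow camera for the Boxcat game that tracks a CameraTarget actor at a set offset.
; Each tick, while the target is valid, it snaps the camera's X and Y to the offset position and eases only the height with FInterpTo.
; It then eases rotation toward a look-at of the target with RInterpTo, sharing CameraSpeed with the height smoothing.
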(event `self.ReceiveTick`
  (params (DeltaSeconds :type "Float (single-precision)"))
  (bind _returnvalue (`GameplayStatics.GetWorldDeltaSeconds`))
  (bind _cameraspeed (`self.CameraSpeed`))
  (bind (_returnvalue_x _returnvalue_y _returnvalue_z) (`KismetMathLibrary.BreakVector` (`SceneComponent.K2_GetComponentLocation` (`self.Camera`))))
  (bind _returnvalue_2 (`self.K2_GetActorLocation` (`self.CameraTarget`)))
  (bind (_returnvalue_x_2 _returnvalue_y_2 _returnvalue_z_2) (`KismetMathLibrary.BreakVector` (+ _returnvalue_2 (`self.CameraOffset`))))
  (`self.CameraTarget`
    (:`then`
      (`SceneComponent.K2_SetWorldLocation` (`self.Camera`) (`KismetMathLibrary.MakeVector` _returnvalue_x_2 _returnvalue_y_2 (`KismetMathLibrary.FInterpTo` _returnvalue_z _returnvalue_z_2 _returnvalue _cameraspeed)) false false)
      (`SceneComponent.K2_SetWorldRotation` (`self.Camera`) (`KismetMathLibrary.RInterpTo` (`SceneComponent.K2_GetComponentRotation` (`self.Camera`)) (`KismetMathLibrary.FindLookAtRotation` (`SceneComponent.K2_GetComponentLocation` (`self.Camera`)) _returnvalue_2) _returnvalue _cameraspeed) false false))
    (:`else`)))

(fn `UserConstructionScript`)